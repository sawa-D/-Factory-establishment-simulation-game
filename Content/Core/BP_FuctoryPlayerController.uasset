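; BP_FuctoryPlayerController is a player controller that puts game-flow UI on screen in response to phase, choice, game-over and game-clear events.
; Each event creates its widget and adds it to the viewport, passing in data such as the phase name, current choice or game-over message.
; The phase banner removes itself after a short delay, while this controller leaves the other screens up.
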(event `self.BP_OnPhaseChanged`
  (params (NewPhase :type "EGamePhase Enum" :default "None"))
  (bind _returnvalue (`|CreateWidget` "/Game/UI/WBP_PhaseBanner.WBP_PhaseBanner_C" self (`|GenericToText` NewPhase)))
  (`UserWidget.AddToViewport` _returnvalue 0)
  (`KismetSystemLibrary.Delay` 2.5)
  (`Widget.RemoveFromParent` _returnvalue))

(event `self.BP_ShowChoiceDialog`
  (params (Choice :type "ChoiceData Object Reference"))
  (bind _returnvalue (`|CreateWidget` "/Game/UI/WBP_ChoiceDialog.WBP_ChoiceDialog_C"))
  (set `/Game/UI/WBP_ChoiceDialog.CurrentChoice` Choice _returnvalue)
  (`UserWidget.AddToViewport` _returnvalue 0))

(event `self.BP_OnGameOver`
  (params (Reason :type "EGameOverReason Enum" :default "None") (Message :type "Text (by ref)"))
  (bind _returnvalue (`|CreateWidget` "/Game/UI/WBP_GameOver.WBP_GameOver_C" self Message))
  (`UserWidget.AddToViewport` _returnvalue 0))

(event `self.BP_OnGameClear`
  (bind _returnvalue (`|CreateWidget` "/Game/UI/WBP_GameClear.WBP_GameClear_C" self))
  (`UserWidget.AddToViewport` _returnvalue 0))

(fn `UserConstructionScript`)